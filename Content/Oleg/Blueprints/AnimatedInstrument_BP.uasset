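; AnimatedInstrument_BP is a collectible instrument actor that registers itself with the level's MetaSoundPlayer when picked up.
; BeginPlay finds that player and binds to the PickUp component's event.
; On pickup, it records its instrument type, updates the music player's instruments and requests a cutscene using materials looked up by type.
; It then removes itself from the first-person character's AllAnimatedObjects list and destroys itself.
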(event `OnPickedUp`
  (params (PickUpCharacter :type "MyProjectCharacter Object Reference"))
  (bind _metasoundplayer (`self.MetaSoundPlayer`))
  (bind _instrument_type (`self.Instrument Type`))
  ;[1 1 1] Add this instrument to Manager(metasound player)
  (`/Engine/EditorBlueprintResources/StandardMacros.IsValid` _metasoundplayer
    (:`Is Valid`
      (`BlueprintMapLibrary.Map_Add` (`/Game/MetaSoundsTool/MetaSoundPlayer.Collected Instruments` _metasoundplayer) _instrument_type true)
      (`/Game/MetaSoundsTool/MetaSoundPlayer.Update_Instruments` _metasoundplayer)
      (`/Game/MetaSoundsTool/MetaSoundPlayer.AddCutsceneToViewport` _metasoundplayer (`self.Get Mat by Instrument Type` _instrument_type) _instrument_type)
      (bind _asbp_first_person_character (cast `/Game/FirstPerson/Blueprints/BP_FirstPersonCharacter` (`Controller.K2_GetPawn` (`GameplayStatics.GetPlayerController` 0))))
      (`KismetArrayLibrary.Array_RemoveItem` (`MyProjectCharacter.AllAnimatedObjects` _asbp_first_person_character) self)
      (`self.K2_DestroyActor`))))

(event `self.ReceiveBeginPlay`
  (`parent.ReceiveBeginPlay`)
  (bind _returnvalue (`GameplayStatics.GetActorOfClass` "/Game/MetaSoundsTool/MetaSoundPlayer.MetaSoundPlayer_C"))
  (set `self.MetaSoundPlayer` _returnvalue)
  (add `PickUp_Component.OnPickUp` (`self.PickUp_`) (delegate `OnPickedUp`)))

(fn `UserConstructionScript`
  (`parent.UserConstructionScript`))