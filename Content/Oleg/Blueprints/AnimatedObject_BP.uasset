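; AnimatedObject is a Blueprint that pulses a mesh's visibility through a dynamic material instance created on BeginPlay.
; TriggerPulse waits a random delay, fades the mesh in, holds for a random duration, fades it out, then blocks re-triggering during a short cooldown.
; Tick advances the shader Time and unclamped fade alphas, writing Time and Visibility to the material.
; SpeedMultiplier scales both the delays and fade rates.
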(event `self.ReceiveBeginPlay`
  (bind _meshcomponent (`self.meshComponent`))
  ;[1 1 1] Create Dynamic Material from Static
  (bind _returnvalue (`PrimitiveComponent.CreateDynamicMaterialInstance` _meshcomponent 0 (`PrimitiveComponent.GetMaterial` _meshcomponent 0) "None"))
  (set `self.DynamicMaterial` _returnvalue))

(event `self.TriggerPulse`
  (params (isEnabled :type Boolean) (minDuration :type "Float (single-precision)") (maxDuration :type "Float (single-precision)"))
  (bind _returnvalue (/ (`KismetMathLibrary.RandomFloatInRange` minDuration maxDuration) (`self.SpeedMultiplier`)))
  ;[1 1 1] Trigger Shader Pulse
  (if isEnabled
    (`KismetSystemLibrary.Delay` (/ (`KismetMathLibrary.RandomFloatInRange` 0.0 1.0) (`self.SpeedMultiplier`)))
    (if (`self.CanPulse`)
      (set `self.CanPulse` false)
      (set `self.Time` 0.0)
      (set `self.InAlpha` 0.0)
      (set `self.IsVisible` true)
      (`KismetSystemLibrary.Delay` _returnvalue)
      (set `self.OutAlpha` 1.0)
      (set `self.IsVisible` false)
      (`KismetSystemLibrary.Delay` (* _returnvalue 0.25))
      (set `self.CanPulse` true))))

(event `self.ReceiveTick`
  (params (DeltaSeconds :type "Float (single-precision)"))
  (bind _returnvalue (* DeltaSeconds (`self.SpeedMultiplier`)))
  ;[1 1 1] Update Shader Time Variable
  (bind _output_get (set `self.Time` (+ DeltaSeconds (`self.Time`))))
  (`MaterialInstanceDynamic.SetScalarParameterValue` (`self.DynamicMaterial`) "Time" _output_get)
  ;[1 1 1] Update fade in alpha value
  (set `self.InAlpha` (+ (`self.InAlpha`) _returnvalue))
  ;[1 1 1] update fade out alpha value
  (set `self.OutAlpha` (- (`self.OutAlpha`) _returnvalue))
  (if (`self.IsVisible`)
    ;[1 1 1] Fade in object
    (`MaterialInstanceDynamic.SetScalarParameterValue` (`self.DynamicMaterial`) "Visibility" (`self.InAlpha`))
    (else
      ;[1 1 1] Fade out object
      (`MaterialInstanceDynamic.SetScalarParameterValue` (`self.DynamicMaterial`) "Visibility" (`self.OutAlpha`)))))

(fn `UserConstructionScript`)