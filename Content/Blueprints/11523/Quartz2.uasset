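; Actor Blueprint that starts Lyre audio playback through the Quartz audio timing subsystem.
; On BeginPlay it creates a named Quartz clock in 4/4, stores the handle, sets a fixed tempo and calls PlayQuantized on Lyre.
; The quantization boundary is None, so playback does not wait for a beat or bar.
; A switch on Bar is left unconnected and never runs.
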(event `self.ReceiveBeginPlay`
  (bind _returnvalue (`QuartzSubsystem.CreateNewClock` (subsystem `QuartzSubsystem`) (`self.Clock Name`) (make `QuartzClockSettings` (make `QuartzTimeSignature` 4)) false true))
  (bind _output_get (set `self.Clock Handle` _returnvalue))
  (`QuartzClockHandle.SetBeatsPerMinute` :`self` _output_get :`BeatsPerMinute` 90.0)
  (`AudioComponent.PlayQuantized` :`self` (`self.Lyre`) :`InClockHandle` (`self.Clock Handle`) :`InQuantizationBoundary` (make `QuartzQuantizationBoundary` "None")))

(fn `UserConstructionScript`)