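; Actor Blueprint that sets up a Quartz clock and starts Lyre music when play begins.
; BeginPlay creates the named clock in 4/4, sets its tempo and calls PlayQuantized on Lyre at a bar-relative dotted-eighth boundary.
; It also spawns Lyre as a 2D sound, stores it as LyreMetasound and zeroes its Period parameter.
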(event `self.ReceiveBeginPlay`
  (bind _returnvalue (`QuartzSubsystem.CreateNewClock` (subsystem `QuartzSubsystem`) (`self.Clock Name`) (make `QuartzClockSettings` (make `QuartzTimeSignature` 4)) false true))
  (bind _output_get (set `self.Clock Handle` _returnvalue))
  (`QuartzClockHandle.SetBeatsPerMinute` :`self` _output_get :`BeatsPerMinute` 90.0)
  (`AudioComponent.PlayQuantized` :`self` (`self.Lyre`) :`InClockHandle` (`self.Clock Handle`) :`InQuantizationBoundary` (make `QuartzQuantizationBoundary` "DottedEighthNote"))
  (bind _returnvalue_2 (`GameplayStatics.SpawnSound2D` "/Game/Blueprints/Lyre.Lyre" 1.0 1.0 0.0 null))
  (bind _output_get_2 (set `self.Lyre Metasound` _returnvalue_2))
  (`AudioParameterControllerInterface.SetFloatParameter` _output_get_2 "Period" 0.0))

(fn `UserConstructionScript`)